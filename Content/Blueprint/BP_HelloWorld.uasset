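; BP_HelloWorld is a DDS publish/subscribe sample that sends and receives a HelloWorld topic.
; On BeginPlay it creates a writer and a reader sharing the same topic settings, QoS and HelloWorld_TopicProxy data type.
; A looping timer sets the proxy's string and float, prints and writes every second.
; The reader's OnDataChanged delegate prints each received string, so the Blueprint acts as both ends of the exchange.
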(event `self.ReceiveBeginPlay`
  (`self.Init Writer`)
  (`self.Init Reader`))

(event `Init Writer`
  ;[1 1 1] DDS Writer Init & Write
  (bind (_topicproxy _writer) (`|CreateWriter` self (make `TopicDescription` (`self.Topic`) (`self.Settings Quality Of Service`)) "/Script/MorseDataModel.HelloWorld_TopicProxy"))
  (set `self.Topic Proxy Writer` _topicproxy)
  (set `self.Writer` _writer)
  (`KismetSystemLibrary.K2_SetTimerDelegate` (delegate `Write`) 1.0 true))

(event `Write`
  (bind _helloworldstr (`self.HelloWorldStr`))
  ;[1 1 1] DDS Writer Init & Write
  (`HelloWorld_TopicProxy.SetData` (`self.Topic Proxy Writer`) (make `MRSHelloWorld` _helloworldstr 40.2))
  (`KismetSystemLibrary.PrintString` (`KismetStringLibrary.Concat_StrStr` "Write : " _helloworldstr))
  (`DDSWriter.Write` (`self.Writer`)))

(event `Init Reader`
  ;[1 1 1] DDS Reader Init & Read
  (bind (_topicproxy _reader) (`|CreateReader` self (make `TopicDescription` (`self.Topic`) (`self.Settings Quality Of Service`)) "/Script/MorseDataModel.HelloWorld_TopicProxy"))
  (set `self.Reader` _reader)
  (bind _output_get (set `self.Topic Proxy_Reader` _topicproxy))
  (add `HelloWorld_TopicProxy.OnDataChanged` _output_get (delegate `OnDataChanged_Event`)))

(event `OnDataChanged_Event`
  (params (Data :type "MRSHelloWorld Structure"))
  ;[1 1 1] DDS Reader Init & Read
  (`KismetSystemLibrary.PrintString` (`KismetStringLibrary.Concat_StrStr` "Read : " Data_Hellostr)))

(fn `UserConstructionScript`)