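; Demo actor that animates itself and publishes its transform over DDS as actor state.
; BeginPlay creates a topic writer and proxy for the ActorState type and stores the starting height.
; Each Tick, ComputeLocation uses a time-based sine to bob Z, increment yaw and pulse clamped scale.
; The new transform is then applied and written to DDS under a hard-coded name and ID.
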(event `self.ReceiveBeginPlay`
  (`self.InitWriter`)
  (set `self.RelativeStartLocationZ` (.z (.location (`self.GetTransform`)))))

(event `InitWriter`
  ;[1 1 1] Init Data Writer
  (bind (_topicproxy _writer) (`|CreateWriter` self (make `TopicDescription` (`self.Topic`)) "/Script/MorseDataModel.ActorState_TopicProxy"))
  (set `self.Topic Proxy` _topicproxy)
  (set `self.Writer` _writer))

(event `Update Actor State`
  ;[1 1 1] Function for set and update the actor state on DDS
  (`ActorState_TopicProxy.SetData` (`self.Topic Proxy`) (make `MRSActorState` "ActorExemple" "1234" (`self.GetTransform`)))
  (`DDSWriter.Write` (`self.Writer`)))

(event `self.ReceiveTick`
  (params (DeltaSeconds :type "Float (single-precision)"))
  ;[1 1 1] Set Actor State
  (bind (_location _rotation _scale) (`self.ComputeLocation`))
  (`self.K2_SetActorTransform` (`KismetMathLibrary.MakeTransform` _location _rotation _scale))
  ;[1 1 1] Update State on DDS
  (`self.Update Actor State`))

(fn `ComputeLocation`
  (returns (Location :type "Vector Structure") (Rotation :type "Rotator Structure") (Scale :type "Vector Structure"))
  (bind (_returnvalue_x _returnvalue_y) (`KismetMathLibrary.BreakVector` (`self.K2_GetActorLocation`)))
  (bind (_returnvalue_roll _returnvalue_pitch _returnvalue_yaw) (`KismetMathLibrary.BreakRotator` (`self.K2_GetActorRotation`)))
  (bind _returnvalue (`KismetMathLibrary.FClamp` (`KismetMathLibrary.DegSin` (* (`self.GetGameTimeSinceCreation`) (`self.BobbingSpeed`))) 0.1))
  (return (`KismetMathLibrary.MakeVector` _returnvalue_x _returnvalue_y (+ (`self.RelativeStartLocationZ`) (* (`KismetMathLibrary.DegSin` (* (`self.GetGameTimeSinceCreation`) (`self.BobbingSpeed`))) (`self.BobbingDistance`)))) (`KismetMathLibrary.MakeRotator` 0.0 0.0 (+ _returnvalue_yaw (`KismetMathLibrary.DegSin` (* (`self.GetGameTimeSinceCreation`) (`self.BobbingSpeed`))))) (`KismetMathLibrary.MakeVector` _returnvalue _returnvalue _returnvalue)))

(fn `UserConstructionScript`)