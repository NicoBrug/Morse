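; BP_HelloWorldPython is a sample actor that publishes HelloWorld messages over DDS.
; On BeginPlay it creates a writer and a HelloWorld_TopicProxy for the configured topic name, then starts a looping one-second timer.
; Each tick of that timer copies the hello string and float variables into the proxy, prints the string to screen and writes the sample.
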(event `self.ReceiveBeginPlay`
  (`self.Init Writer`))

(event `Init Writer`
  ;[1 1 1] DDS Writer Init & Write
  (bind (_topicproxy _writer) (`|CreateWriter` self (make `TopicDescription` (`self.TopicName`)) "/Script/MorseDataModel.HelloWorld_TopicProxy"))
  (set `self.Topic Proxy Writer` _topicproxy)
  (set `self.Writer` _writer)
  (`KismetSystemLibrary.K2_SetTimerDelegate` (delegate `Write`) 1.0 true))

(event `Write`
  (bind _helloworldstr (`self.HelloWorldStr`))
  ;[1 1 1] DDS Writer Init & Write
  (`HelloWorld_TopicProxy.SetData` (`self.Topic Proxy Writer`) (make `MRSHelloWorld` _helloworldstr (`self.HelloWorldFloat`)))
  (`KismetSystemLibrary.PrintString` (`KismetStringLibrary.Concat_StrStr` "Write : " _helloworldstr))
  (`DDSWriter.Write` (`self.Writer`)))

(fn `UserConstructionScript`)